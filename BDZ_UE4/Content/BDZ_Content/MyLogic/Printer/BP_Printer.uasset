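; BP_Printer is a 3D printer actor that animates a print job and spawns the printed part.
; Its Printer event loops the skeletal mesh animation for a given time, stops it, then spawns the passed object's class at the printer's location.
; Disconnected logic would read a start flag and object number from the game instance to pick one of seven parts and its print time, but Tick is empty, so it never runs.
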(event `self.ReceiveTick`
  (params (DeltaSeconds :type "Float (single-precision)")))

(event `Printer`
  (params (Object :type "Actor Object Reference") (Time :type "Float (double-precision)"))
  (`SkeletalMeshComponent.PlayAnimation` (`self.SKM_3D_printer`) "/Game/BDZ_Content/Models_and_other/3D_Printer/AS_3D_printer_anim.AS_3D_printer_anim" true)
  (`KismetSystemLibrary.Delay` Time)
  (`SkeletalMeshComponent.Stop` (`self.SKM_3D_printer`))
  (`|SpawnActorFromClass` (`GameplayStatics.GetObjectClass` Object) (`KismetMathLibrary.MakeTransform` (`self.K2_GetActorLocation`)) "Undefined" "OverrideRootScale" null null))

(fn `UserConstructionScript`)