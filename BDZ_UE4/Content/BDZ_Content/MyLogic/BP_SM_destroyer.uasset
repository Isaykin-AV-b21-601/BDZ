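; BP_SM_destroyer is an overlap trigger that destroys grabbable objects and ends the task once enough are removed.
; Each overlapping BP_GrabObject is destroyed and counted.
; When the count reaches exactly 21, it spawns a BP_Robot at a fixed location, creates the W_Final widget if FinalWiget is not valid, shows the mouse cursor and adds the widget to the viewport.
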(event `self.ReceiveActorBeginOverlap`
  (params (OtherActor :type "Actor Object Reference"))
  (cast `/Game/BDZ_Content/MyLogic/Grab/BP_GrabObject` OtherActor)
  (set `self.DeletedOnbjectsCount` (+ (`self.DeletedOnbjectsCount`) 1))
  (`self.K2_DestroyActor` OtherActor)
  (if (== (`self.DeletedOnbjectsCount`) 21)
    (`|SpawnActorFromClass` "/Game/BDZ_Content/MyLogic/BP_Robot.BP_Robot_C" (`KismetMathLibrary.MakeTransform` (-2080.0 1370.0 270.0)) "Undefined" "OverrideRootScale" null null)
    (`/Engine/EditorBlueprintResources/StandardMacros.IsValid` (`self.FinalWiget`)
      (:`Is Valid`
        _)
      (:`Is Not Valid`
        (bind _returnvalue (`|CreateWidget` "/Game/BDZ_Content/Widgets/W_Final.W_Final_C"))))
    (set `PlayerController.bShowMouseCursor` true (`GameplayStatics.GetPlayerController` 0))
    (`UserWidget.AddToViewport` _returnvalue 0)))

(fn `UserConstructionScript`)