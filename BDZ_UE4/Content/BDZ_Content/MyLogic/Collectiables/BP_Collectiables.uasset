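; Collectible item actor that shows a floating name label and goes into the player's inventory on interaction.
; At BeginPlay it writes its Name into the widget component's text block and hides it; Showtext reveals it and yaws it once toward the player.
; Interaction increments this class's count in FirstPersonCharacter's parallel Inventory and InvenoryItemCount arrays, or appends a new entry, then destroys the actor.
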(event `Hide text`
  ;[1 1 1] Показать/скрыть текст
  (`Widget.SetVisibility` (`self.TextBlock`) "Hidden"))

(event `self.ReceiveBeginPlay`
  ;[1 1 1] Подписи для объектов
  (bind _asw_identificator_for_interaction (cast `/Game/BDZ_Content/Widgets/W_Identificator_for_interaction` (`WidgetComponent.GetUserWidgetObject` (`self.Widget`))))
  (bind _objectname (`/Game/BDZ_Content/Widgets/W_Identificator_for_interaction.Objectname` _asw_identificator_for_interaction))
  (`TextBlock.SetText` _objectname (`KismetTextLibrary.Conv_StringToText` (`self.Name`)))
  (set `self.TextBlock` _objectname)
  (`self.Hide text`))

(event `Show text`
  (bind _widget (`self.Widget`))
  (bind (_returnvalue_roll _returnvalue_pitch _returnvalue_yaw) (`KismetMathLibrary.BreakRotator` (`KismetMathLibrary.FindLookAtRotation` (`SceneComponent.K2_GetComponentLocation` _widget) (`self.K2_GetActorLocation` (`GameplayStatics.GetPlayerCharacter` 0)))))
  ;[1 1 1] Показать/скрыть текст
  (`Widget.SetVisibility` (`self.TextBlock`) "Visible")
  ;[1 1 1] Поворот текста за игроком
  (`SceneComponent.K2_SetWorldRotation` _widget (`KismetMathLibrary.MakeRotator` 0.0 0.0 _returnvalue_yaw) false false))

(event `/Game/BDZ_Content/Widgets/BP_Interaction.interaction`
  (bind _returnvalue (`GameplayStatics.GetObjectClass` self))
  ;[1 1 1] Заполнение инвентаря предметами и подсчёт
  (bind _asfirst_person_character (cast `/Game/FirstPersonBP/Blueprints/FirstPersonCharacter` (`GameplayStatics.GetPlayerCharacter` 0)))
  (bind _inventory (`/Game/FirstPersonBP/Blueprints/FirstPersonCharacter.Inventory` _asfirst_person_character))
  (if (`KismetArrayLibrary.Array_Contains` _inventory _returnvalue)
    (bind _invenory_item_count (`/Game/FirstPersonBP/Blueprints/FirstPersonCharacter.Invenory_item_count` _asfirst_person_character))
    (bind _returnvalue_2 (`KismetArrayLibrary.Array_Find` _inventory _returnvalue))
    (`KismetArrayLibrary.Array_Set` _invenory_item_count _returnvalue_2 (+ (`|GetArrayItem` _invenory_item_count _returnvalue_2) 1))
    (else
      (`KismetArrayLibrary.Array_Add` _inventory _returnvalue)
      (`KismetArrayLibrary.Array_Add` _invenory_item_count 1)))
  (`self.K2_DestroyActor`))

(fn `UserConstructionScript`)